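; BP_Moveing is a moving platform that travels in a straight line toward an EndPoint component, which is hidden when play begins.
; Each Tick it normalizes the vector from PlatformMesh to EndPoint and adds it to the mesh's world location, without sweep.
; The step is one unit per frame, so speed depends on frame rate, and there is no arrival check or return trip.
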(event EventBeginPlay
  (|CallParentFunction)
  (Development|SetHiddeninGame (Variables|Default|GetEndPoint) true false))

(event Collision|EventActorBeginOverlap
  (params (OtherActor :type Actor%20Object%20Reference))
  (|CallParentFunction OtherActor) ; 지금 이 노드는 비활성 상태입니다. \n핀을 끌어서 다른 노드를 연결하면 활성화됩니다.
)

(event EventTick
  (params (DeltaSeconds :type Float%20%28single-precision%29))
  (bind _platformmesh (Variables|Default|GetPlatformMesh))
  (bind _returnvalue (Transformation|GetWorldLocation _platformmesh))
  (|CallParentFunction DeltaSeconds)
  (Transformation|SetWorldLocation _platformmesh (+ (Math|Vector|Normalize (- (Transformation|GetWorldLocation (Variables|Default|GetEndPoint)) _returnvalue)) _returnvalue) false false))

(fn ConstructionScript
  (|CallParentFunction))