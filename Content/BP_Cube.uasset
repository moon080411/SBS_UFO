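; BP_Cube is an actor that moves and rotates continuously, apparently as a basic transform exercise.
; BeginPlay prints the starting location, offsets it along world X and sets a fixed rotation.
; Tick steps it further along X without delta-time scaling, so speed depends on frame rate.
; Each tick also sets roll, pitch and yaw all to the current yaw plus a fixed increment.
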(event EventBeginPlay
  (Development|PrintString (Utilities|String|ToString(Vector) (Transformation|GetActorLocation)))
  (Transformation|SetActorLocation (+ (Transformation|GetActorLocation) "300.000000,0.000000,0.000000") false false) ; 위치 변경
  (Transformation|SetActorRotation "90.000000,0.000000,0.000000") ; 회전 변경
)

(event EventTick
  (params (DeltaSeconds :type Float%20%28single-precision%29))
  (bind _returnvalue (Transformation|GetActorRotation))
  (bind _returnvalue_2 (+ (.yaw _returnvalue) 17.0))
  (Transformation|SetActorLocation (+ (Transformation|GetActorLocation) "17.000000,0.000000,0.000000") false false) ; 위치 변경
  (Transformation|SetActorRotation (Math|Rotator|MakeRotator _returnvalue_2 _returnvalue_2 _returnvalue_2)) ; 회전 변경
)

(fn ConstructionScript)